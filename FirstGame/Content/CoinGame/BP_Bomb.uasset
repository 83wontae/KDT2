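; BP_Bomb is a proximity-triggered bomb that counts down and explodes, knocking player characters away.
; Any overlap with the Detect component reveals a text countdown, which Tick advances for ten seconds before calling DoBomb.
; DoBomb ragdolls each BP_ThirdPersonCharacter in the Damage volume and applies an outward mesh impulse that weakens with clamped distance.
; It then spawns an explosion emitter and destroys itself.
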(event OnComponentBeginOverlap(detect)
  (params (OverlappedComponent :type Primitive%20Component%20Object%20Reference) (OtherActor :type Actor%20Object%20Reference) (OtherComp :type Primitive%20Component%20Object%20Reference) (OtherBodyIndex :type Integer) (bFromSweep :type Boolean) (SweepResult :type Hit%20Result%20Structure%20%28by%20ref%29))
  (CallFunction|DoDetect))

(event EventTick
  (params (DeltaSeconds :type Float%20%28single-precision%29))
  (if (Variables|Default|GetIsDetact)
    (bind _output_get (Variables|Default|SetTotalTime (+ DeltaSeconds (Variables|Default|GetTotalTime))))
    (Rendering|Components|TextRender|SetText (Variables|Default|GetTextRender) (Utilities|Text|ToText(Integer) (- 10 (Math|Float|Floor _output_get))))
    (if (> (Variables|Default|GetTotalTime) 1e+01)
      (CallFunction|DoBomb))))

(event EventBeginPlay
  (Rendering|SetVisibility (Variables|Default|GetTextRender) false false))

(fn ConstructionScript)

(fn DoBomb
  (Development|PrintString "Bomb")
  (for _array_element (Collision|GetOverlappingActors (Variables|Default|Getdamage) "/Game/ThirdPerson/Blueprints/BP_ThirdPersonCharacter.BP_ThirdPersonCharacter_C" :!class /Script/Engine.PrimitiveComponent)
    (bind _asbp_third_person_character (Utilities|Casting|CastToBP_ThirdPersonCharacter _array_element))
    (CallFunction|PushCharacter _asbp_third_person_character))
  (Effects|SpawnEmitteratLocation "/Game/StarterContent/Particles/P_Explosion.P_Explosion" (Transformation|GetActorLocation) (Transformation|GetActorRotation) "5.000000,5.000000,5.000000")
  (Actor|DestroyActor))

(fn PushCharacter
  (params (Character :type BP%20Third%20Person%20Character%20Object%20Reference))
  (Default|DoRagdoll Character)
  (Physics|AddImpulse (Variables|/Script/Engine.Character|GetMesh Character) (* (Math|Vector|GetForwardVector (Math|Rotator|FindLookatRotation (Transformation|GetActorLocation) (Transformation|GetActorLocation Character))) (/ (Variables|Default|GetMaxImpulse) (Math|Float|Clamp(Float) (* (Math|Vector|Distance(Vector) (Transformation|GetActorLocation Character) (Transformation|GetActorLocation)) 0.01) 1.0 5.0))) "None" false))

(fn DoDetect
  (Variables|Default|SetIsDetact true)
  (Rendering|SetVisibility (Variables|Default|GetTextRender) true false))