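; BP_Arrow is a physics-driven arrow projectile in CoinGame that destroys itself five seconds after BeginPlay.
; BeginPlay launches the mesh forward with an impulse randomized within a narrow cone.
; Tick turns the actor to face its velocity until IsHit is set.
; A hit or overlap stops physics and collision, with overlaps also attaching the arrow to the other component in place.
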(event OnComponentHit(SM_Arrow)
  (params (HitComponent :type Primitive%20Component%20Object%20Reference) (OtherActor :type Actor%20Object%20Reference) (OtherComp :type Primitive%20Component%20Object%20Reference) (NormalImpulse :type Vector :default "0, 0, 0") (Hit :type Hit%20Result%20Structure%20%28by%20ref%29))
  (Variables|Default|SetisHit true)
  (Physics|SetSimulatePhysics (Variables|Default|GetSM_Arrow) false)
  (Collision|SetCollisionEnabled (Variables|Default|GetSM_Arrow) "NoCollision"))

(event OnComponentBeginOverlap(SM_Arrow)
  (params (OverlappedComponent :type Primitive%20Component%20Object%20Reference) (OtherActor :type Actor%20Object%20Reference) (OtherComp :type Primitive%20Component%20Object%20Reference) (OtherBodyIndex :type Integer) (bFromSweep :type Boolean) (SweepResult :type Hit%20Result%20Structure%20%28by%20ref%29))
  (Variables|Default|SetisHit true)
  (Physics|SetSimulatePhysics (Variables|Default|GetSM_Arrow) false)
  (Collision|SetCollisionEnabled (Variables|Default|GetSM_Arrow) "NoCollision")
  (Transformation|AttachComponentToComponent OtherComp "None" "KeepWorld" "KeepWorld" "KeepWorld" true))

(event EventBeginPlay
  (bind _sm_arrow (Variables|Default|GetSM_Arrow))
  (Physics|AddImpulse _sm_arrow (* (Math|Random|RandomUnitVectorinConeinDegrees (Math|Vector|GetForwardVector _sm_arrow) 1e+01) 1e+03) "None" false)
  (Utilities|FlowControl|Delay 5.0)
  (Actor|DestroyActor))

(event EventTick
  (params (DeltaSeconds :type Float%20%28single-precision%29))
  (if (not (Variables|Default|GetisHit))
    (Transformation|SetActorRotation (Math|Conversions|RotationFromXVector (Transformation|GetComponentVelocity (Variables|Default|GetSM_Arrow))))))

(fn ConstructionScript)